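; Lobby player controller that spawns the player in VR or non-VR mode based on saved settings.
; On BeginPlay, ClientBeginPlay loads the PlayerSaveGame slot and reads its VRMode flag.
; It passes that flag and player controller 0 to InitiateSpawnPlayer, which delegates spawning to LobbyGMM, then enables or disables the HMD to match.
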(event `InitiateSpawnPlayer`
  (params (`IsVRMode?` :type Boolean) (NewPlayer :type "PlayerController Object Reference"))
  (`KismetSystemLibrary.PrintString` "Hello")
  (bind _aslobby_gmm (cast `/Game/Blueprints/Lobby/LobbyGMM` (`GameplayStatics.GetGameMode`)))
  (`/Game/Blueprints/Lobby/LobbyGMM.SpawnPlayer` _aslobby_gmm NewPlayer `IsVRMode?`))

(event `self.ReceiveBeginPlay`
  (`self.ClientBeginPlay`))

(event `ClientBeginPlay`
  (bind _returnvalue (`GameplayStatics.LoadGameFromSlot` (`self.PlayerSettingsSave`)))
  (bind _asplayer_save_game (cast `/Game/Blueprints/AllLevels/PlayerSaveGame` _returnvalue))
  (bind (_myplayername _myplayerstatus _myplayerimage _myplayercharacter _myplayercharacterimage _vrmode_) (break `/Game/Blueprints/AllLevels/PlayerInfo` (`/Game/Blueprints/AllLevels/PlayerSaveGame.S_PlayerInfo` _asplayer_save_game)))
  (`self.InitiateSpawnPlayer` _vrmode_ (`GameplayStatics.GetPlayerController` 0))
  (`HeadMountedDisplayFunctionLibrary.EnableHMD` _vrmode_))

(fn `UserConstructionScript`)