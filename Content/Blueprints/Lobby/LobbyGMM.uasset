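; Lobby game mode that picks the player's pawn type from a saved VR setting.
; Its SpawnDefaultPawnFor override loads the PlayerSettingsSave slot and, in VR mode, enables the HMD and spawns a MotionControllerPawn at the start spot; otherwise it spawns a Barberous there.
; No pawn is spawned if the save fails to cast to PlayerSaveGame, and an HMD device-name check is left unconnected.
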(fn `SpawnDefaultPawnFor`
  (params (NewPlayer :type "Controller Object Reference") (StartSpot :type "Actor Object Reference"))
  (returns (ReturnValue :type "Pawn Object Reference"))
  (bind _returnvalue (`self.GetTransform` StartSpot))
  (bind _returnvalue_2 (`GameplayStatics.LoadGameFromSlot` (`self.PlayerSettingsSave`)))
  (bind _asplayer_save_game (cast `/Game/Blueprints/AllLevels/PlayerSaveGame` _returnvalue_2))
  (if (`.VRMode?_15_F0EEDBC846F837C6D4D762A6E4991588` (break `/Game/Blueprints/AllLevels/PlayerInfo` (`/Game/Blueprints/AllLevels/PlayerSaveGame.S_PlayerInfo` _asplayer_save_game)))
    (`HeadMountedDisplayFunctionLibrary.EnableHMD` true)
    (bind _returnvalue_3 (`|SpawnActorFromClass` "/Game/VirtualRealityBP/Blueprints/MotionControllerPawn.MotionControllerPawn_C" _returnvalue "Undefined" "OverrideRootScale"))
    (return _returnvalue_3)
    (else
      (bind _returnvalue_4 (`|SpawnActorFromClass` "/Game/Blueprints/Characters/Barberous.Barberous_C" _returnvalue "Undefined" "OverrideRootScale"))
      (return _returnvalue_4))))

(fn `UserConstructionScript`)